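; Third-person shooter player Blueprint for a character with a grenade gun and a sniper, currently inert: every event and function body is empty.
; Disconnected nodes hold the intended logic for movement, look, jump, weapon visibility swapping, crosshair and sniper UI, and FOV zoom.
; Also unwired, firing either spawns bullet actors at a muzzle socket or line-traces from the camera, adding explosion effects and mass-scaled force to physics objects.
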(event `InputAction|SniperGun` :overrideparent false
  (params (Key :type "Key Structure")))

(event `InputAction|GrenadeGun` :overrideparent false
  (params (Key :type "Key Structure")))

(event `self.ReceiveBeginPlay`)

(event `ChangeGun`
  (params (bShowGrenade :type Boolean))
  ;[0.4623 0.476 1] Comment
)

(event `InputAction|Zoom` :overrideparent false
  (params (Key :type "Key Structure")))

(event `InputAxis|Turn Right` :overrideparent false
  (params (AxisValue :type "Float (single-precision)")))

(event `self.ReceiveTick`
  (params (DeltaSeconds :type "Float (single-precision)"))
  ;[1 1 1] P=P0+vt 이동 등가속도공식
)

(event `InputAxis|Look Up` :overrideparent false
  (params (AxisValue :type "Float (single-precision)")))

(event `InputAction|Fire` :overrideparent false
  (params (Key :type "Key Structure")))

(event `InputAction|Jump` :overrideparent false
  (params (Key :type "Key Structure")))

(fn `SetGunUI`
  (params (bGrenadeGun :type Boolean)))

(fn `UserConstructionScript`)